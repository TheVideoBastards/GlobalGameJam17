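; A portal door that teleports any overlapping actor to its linked portal.
; On overlap, if LinkedPortal is set, it moves the actor to the position and rotation of that portal's first Arrow component, which serves as the exit point.
; It also sets player controller 0's control rotation to the arrow's rotation, regardless of which actor entered.
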(event Collision|EventActorBeginOverlap
  (params (OtherActor :type Actor%20Object%20Reference))
  (bind _linkedportal (Variables|Default|GetLinkedPortal))
  (bind _returnvalue (Actor|GetComponentsByClass _linkedportal "/Script/Engine.ArrowComponent"))
  (bind _item (Utilities|Array|Get(acopy) _returnvalue))
  (bind _returnvalue_2 (Transformation|GetWorldRotation _item))
  (if (!= _linkedportal 0)
    (Transformation|SetActorLocationAndRotation OtherActor (Transformation|GetWorldLocation _item) _returnvalue_2 false true)
    (Pawn|SetControlRotation (Game|GetPlayerController 0) _returnvalue_2)))

(fn ConstructionScript
  (|CallParentFunction))